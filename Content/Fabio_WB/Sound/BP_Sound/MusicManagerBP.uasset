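; Music manager that holds the level's tracks and switches which one is audible.
; On BeginPlay it creates a 2D sound for each TrackList entry, starts all of them muted, then raises the SongOnLevelBegin track to MusicVolume.
; ChangeMusicto mutes the current track and unmutes the requested index instantly, with no fade or restart, and prints a debug message.
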(event `self.ReceiveBeginPlay`
  (bind _output (`|GetArrayItem` (`self.MusicRefferences`) (`self.Song on Level Begin`)))
  (for _array_element (`self.TrackList`)
    (bind _returnvalue (`GameplayStatics.CreateSound2D` _array_element 1.0 1.0 0.0 null))
    (`KismetArrayLibrary.Array_Add` (`self.MusicRefferences`) _returnvalue)
    (`AudioComponent.SetVolumeMultiplier` _returnvalue 0.0)
    (`AudioComponent.Play` _returnvalue 0.0))
  (`AudioComponent.SetVolumeMultiplier` _output (`self.Music Volume`))
  (set `self.Current Music Ref` _output))

(event `Change Music to`
  (params (IndexOfSongToPlay :type Integer))
  (bind _output (`|GetArrayItem` (`self.MusicRefferences`) IndexOfSongToPlay))
  (`AudioComponent.SetVolumeMultiplier` (`self.Current Music Ref`) 0.0)
  (`AudioComponent.SetVolumeMultiplier` _output (`self.Music Volume`))
  (bind _output_get (set `self.Current Music Ref` _output))
  (`KismetSystemLibrary.PrintString` (`KismetStringLibrary.Concat_StrStr` "music playing" (`KismetSystemLibrary.GetDisplayName` _output_get))))

(fn `UserConstructionScript`)