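; BP_Muelleimer is a trash can that disposes of the item the player is holding.
; Its Wegwergen? event runs only if the passed object is a BP_Item, then reads HoldingItem from BP_Player rather than using that object.
; It detaches the held item, snaps it to ItemLocation, clears the player's reference and destroys the item immediately.
; A 2D splash sound then plays from an offset start time.
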(event `Wegwergen?`
  (params (B :type "Object Object Reference"))
  (cast `/Game/Juli_WB/Blueprints/BP_Item` B)
  (bind _asbp_player (cast `/Game/Juli_WB/BP_Player` (`GameplayStatics.GetPlayerCharacter` 0)))
  (bind _holdingitem (`/Game/Juli_WB/BP_Player.HoldingItem` _asbp_player))
  (`self.K2_DetachFromActor` _holdingitem "KeepWorld" "KeepWorld" "KeepWorld")
  (`self.K2_AttachToComponent` _holdingitem (`self.ItemLocation`) "None" "SnapToTarget" "KeepWorld" "KeepWorld" true)
  (bind _output_get (set `self.Item` _holdingitem))
  (set `/Game/Juli_WB/BP_Player.HoldingItem` null _asbp_player)
  (`self.K2_DestroyActor` _output_get)
  (`GameplayStatics.PlaySound2D` "/Game/WB_Mow/Sounds/SFX/splash-by-blaukreuz-6261_Cue.splash-by-blaukreuz-6261_Cue" 1.0 1.0 1.0 null null))

(fn `UserConstructionScript`)