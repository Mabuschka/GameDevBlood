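; Corpse actor that players chop with a tool to harvest an organ.
; Each Chop call spawns blood splash, advances Progress by delta time and shows the progress widget, which a retriggerable delay hides once chopping pauses.
; At full progress it spawns a chopped corpse, destroys itself and pops out a randomly tilted organ chosen by tool flag: machete lung, hammer brain, saw heart, scissors intestine, spoon eyes.
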(event `self.ReceiveBeginPlay`
  (bind _aswidget_progress (cast `/Game/Juli_WB/Blueprints/Widget_Progress` (`WidgetComponent.GetUserWidgetObject` (`self.Widget`))))
  (set `self.As Widget Progress` _aswidget_progress))

(event `Chop`
  (params (`Delta Time` :type "Float (double-precision)") (`Machete?` :type Boolean) (Hammer :type Boolean) (Saege :type Boolean) (Schere :type Boolean) (Spoon :type Boolean))
  (bind _returnvalue_location (`KismetMathLibrary.BreakTransform` (`self.GetTransform`)))
  (bind _returnvalue (`KismetMathLibrary.RandomFloatInRange` -40.0 40.0))
  (bind _returnvalue_2 (`KismetMathLibrary.RandomFloatInRange` -40.0 40.0))
  (bind _progress (`self.Progress`))
  (bind _returnvalue_3 (+ _returnvalue_location (0.0 0.0 150.0)))
  (`NiagaraFunctionLibrary.SpawnSystemAtLocation` "/Game/Juli_WB/Assets/Materials/FX/BlodSplash.BlodSplash" (`self.K2_GetActorLocation`))
  (set `/Game/Juli_WB/Blueprints/Widget_Progress.Progress` _progress (`self.As Widget Progress`))
  (if (< _progress 1.0)
    (set `self.Progress` (+ (`self.Progress`) (* `Delta Time` 0.5)))
    (`SceneComponent.SetVisibility` (`self.Widget`) true false)
    (`KismetSystemLibrary.RetriggerableDelay` 0.15)
    (`SceneComponent.SetVisibility` (`self.Widget`) false false)
    (else
      (`|SpawnActorFromClass` (`self.ChoppedLeiche`) (`self.GetTransform`) "Undefined" "OverrideRootScale" null null)
      (`self.K2_DestroyActor`)
      (if `Machete?`
        (`|SpawnActorFromClass` "/Game/Juli_WB/Blueprints/BP_Lunge.BP_Lunge_C" (`KismetMathLibrary.MakeTransform` _returnvalue_3 (`KismetMathLibrary.MakeRotator` _returnvalue _returnvalue_2) (0.825 1.222768 0.825)) "Undefined" "OverrideRootScale" null null)
        (elif Hammer
          (`|SpawnActorFromClass` "/Game/Juli_WB/Blueprints/BP_Brain.BP_Brain_C" (`KismetMathLibrary.MakeTransform` _returnvalue_3 (`KismetMathLibrary.MakeRotator` _returnvalue _returnvalue_2) (0.9 0.9 0.9)) "Undefined" "OverrideRootScale" null null)
          (elif Saege
            (`|SpawnActorFromClass` "/Game/Juli_WB/Blueprints/BP_Heart.BP_Heart_C" (`KismetMathLibrary.MakeTransform` _returnvalue_3 (`KismetMathLibrary.MakeRotator` _returnvalue _returnvalue_2)) "Undefined" "OverrideRootScale" null null)
            (elif Schere
              (`|SpawnActorFromClass` "/Game/Juli_WB/Blueprints/BP_Darm.BP_Darm_C" (`KismetMathLibrary.MakeTransform` _returnvalue_3 (`KismetMathLibrary.MakeRotator` _returnvalue _returnvalue_2) (1.5 1.5 1.5)) "Undefined" "OverrideRootScale" null null)
              (elif Spoon
                (`|SpawnActorFromClass` "/Game/Juli_WB/Blueprints/BP_Eyes.BP_Eyes_C" (`KismetMathLibrary.MakeTransform` _returnvalue_3 (`KismetMathLibrary.MakeRotator` _returnvalue _returnvalue_2) (0.7 0.7 0.7)) "Undefined" "OverrideRootScale" null null)))))))))

(fn `UserConstructionScript`)