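; BP_Abgabe is an organ drop-off point that scores the item the player delivers and creates the Widget_Punkte HUD on BeginPlay.
; RichtigesItem? casts the passed item to each of five organ classes and compares it with the player's OrganNr, adding points on a match and deducting on a mismatch.
; Both outcomes share one tail that moves the held item to ItemLocation, destroys it, resets OrganNr and calls NewQuest on the widget.
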(event `RichtigesItem?`
  (params (B :type "Object Object Reference"))
  (bind _asbp_player (cast `/Game/Juli_WB/BP_Player` (`GameplayStatics.GetPlayerCharacter` 0)))
  (`|ExecutionSequence`
    (:`then_0`
      (cast `/Game/Juli_WB/Blueprints/BP_Brain` B)
      (bind _organnr (`/Game/Juli_WB/BP_Player.OrganNr` _asbp_player))
      (if (== _organnr 0)
        (bind _score (`/Game/Juli_WB/BP_Player.Score` _asbp_player))
        (set `/Game/Juli_WB/BP_Player.Score` (+ _score 10) _asbp_player :!label _label)
        (else
          (set `/Game/Juli_WB/BP_Player.Score` (- _score 5) _asbp_player :!label _label_2))))
    (:`then_1`
      (cast `/Game/Juli_WB/Blueprints/BP_Darm` B)
      (if (== _organnr 1)
        (goto _label)
        (else
          (goto _label_2))))
    (:`then_2`
      (cast `/Game/Juli_WB/Blueprints/BP_Lunge` B)
      (if (== _organnr 2)
        (goto _label)
        (else
          (goto _label_2))))
    (:`then_3`
      (cast `/Game/Juli_WB/Blueprints/BP_Eyes` B)
      (if (== _organnr 3)
        (goto _label)
        (else
          (goto _label_2))))
    (:`then_4`
      (cast `/Game/Juli_WB/Blueprints/BP_Heart` B)
      (if (== _organnr 4)
        (goto _label)
        (else
          (goto _label_2)))))
  (bind _holdingitem (`/Game/Juli_WB/BP_Player.HoldingItem` _asbp_player))
  (`self.K2_DetachFromActor` _holdingitem "KeepWorld" "KeepWorld" "KeepWorld")
  (`self.K2_AttachToComponent` _holdingitem (`self.ItemLocation`) "None" "SnapToTarget" "KeepWorld" "KeepWorld" true)
  (bind _output_get (set `self.Item` _holdingitem))
  (set `/Game/Juli_WB/BP_Player.HoldingItem` null _asbp_player)
  (`self.K2_DestroyActor` _output_get)
  (set `/Game/Juli_WB/BP_Player.OrganNr` 5 _asbp_player)
  (`/Game/Juli_WB/QuestSystem/Widget_Punkte.NewQuest` (stale `self.ReceiveBeginPlay` _returnvalue)))

(event `self.ReceiveBeginPlay`
  (bind _returnvalue (`|CreateWidget` "/Game/Juli_WB/QuestSystem/Widget_Punkte.Widget_Punkte_C"))
  (`UserWidget.AddToViewport` _returnvalue 0))

(fn `UserConstructionScript`)