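; Player pawn that walks on world axes, carries items between desks and chops corpses on chopping tables with one of five tools.
; Tick turns the mesh toward movement input, spawns running effects and box-traces ahead for the interaction target, with debug drawing and printing.
; Pickup/Drop swaps items with desks or grabs loose ones, setting per-tool rotations.
; Holding Chop opens a gate that calls the corpse's Chop every frame, blocking pickup meanwhile.
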(event `InputAxis|MoveForward`
  (params (AxisValue :type "Float (single-precision)"))
  (`self.AddMovementInput` (1.0 0.0 0.0) AxisValue))

(event `InputAction|pickUp/Drop`
  (params (Key :type "Key Structure"))
  (:`Pressed`
    (if (not (`self.isChopping`))
      (`self.DeskFunctions` (`.HitActor` (`GameplayStatics.BreakHitResult` (stale `self.ReceiveTick` _outhit)))))))

(event `InputAxis|MoveRight`
  (params (AxisValue :type "Float (single-precision)"))
  (`self.AddMovementInput` (0.0 1.0 0.0) AxisValue))

(event `InputAction|Chop`
  (params (Key :type "Key Structure"))
  (bind _returnvalue (== (`self.HoldingItem`) (`self.Spoon`)))
  (bind _returnvalue_2 (== (`self.HoldingItem`) (`self.Machete`)))
  (bind _returnvalue_3 (== (`self.HoldingItem`) (`self.Hammer`)))
  (bind _returnvalue_4 (== (`self.HoldingItem`) (`self.Saege`)))
  (bind _returnvalue_5 (== (`self.HoldingItem`) (`self.Schere`)))
  (:`Pressed`
    (goto _label :!via `Open`))
  (:`Released`
    (set `self.isChopping` false)
    (goto _label :!via `Close`)))

(event `self.ReceiveTick`
  (params (DeltaSeconds :type "Float (single-precision)"))
  (bind _mesh (`self.Mesh`))
  (bind _returnvalue (`SceneComponent.K2_GetComponentLocation` _mesh))
  (bind _returnvalue_2 (== (`self.HoldingItem`) (`self.Spoon`)))
  (bind _returnvalue_3 (== (`self.HoldingItem`) (`self.Machete`)))
  (bind _returnvalue_4 (== (`self.HoldingItem`) (`self.Hammer`)))
  (bind _returnvalue_5 (== (`self.HoldingItem`) (`self.Saege`)))
  (bind _returnvalue_6 (== (`self.HoldingItem`) (`self.Schere`)))
  (bind _returnvalue_7 (`KismetMathLibrary.RLerp` (`SceneComponent.K2_GetComponentRotation` (`self.Mesh`)) (`KismetMathLibrary.Conv_VectorToRotator` (`self.direction`)) (* DeltaSeconds (`self.rotationSpeed`)) true))
  (`|ExecutionSequence`
    (:`then_0`
      (`KismetSystemLibrary.PrintString` (`KismetSystemLibrary.GetDisplayName` (`self.HoldingItem`)) true true (struct :`G` 0.66 :`B` 1.0 :`A` 1.0) 0.0)
      (`KismetSystemLibrary.PrintString` (`KismetStringLibrary.Conv_BoolToString` (`self.isChopping`)) true true (struct :`G` 0.66 :`B` 1.0 :`A` 1.0) 0.0))
    (:`then_1`
      (if (or (!= (`self.GetInputAxisValue`) 0.0) (!= (`self.GetInputAxisValue`) 0.0))
        (`NiagaraFunctionLibrary.SpawnSystemAtLocation` "/Game/Juli_WB/Assets/Materials/FX/Running.Running" (+ (`self.K2_GetActorLocation`) (0.0 0.0 -75.0)) _returnvalue_7)
        (set `self.direction` (`KismetMathLibrary.MakeVector` (`self.GetInputAxisValue`) (* -1 (`self.GetInputAxisValue`))))
        (`SceneComponent.K2_SetWorldRotation` _mesh _returnvalue_7 false false))
      (bind _outhit (`KismetSystemLibrary.BoxTraceSingle` :`Start` _returnvalue :`End` (+ _returnvalue (* (`SceneComponent.GetRightVector` _mesh) (`self.reachDistance`))) :`HalfSize` (`self.Half Size`) :`TraceChannel` "TraceTypeQuery1" :`DrawDebugType` "ForOneFrame"))
      (`/Engine/EditorBlueprintResources/StandardMacros.Gate` true :!label _label
        (:`Exit`
          (bind _asbp_choping_table (cast `/Game/Juli_WB/Blueprints/BP_ChopingTable` (`.HitActor` (`GameplayStatics.BreakHitResult` _outhit)))
            (:`then`
              (bind _asbp_leiche (cast `/Game/Juli_WB/Blueprints/BP_Leiche` (`/Game/Juli_WB/Blueprints/BP_ChopingTable.Corpse` _asbp_choping_table))
                (:`then`
                  (if (`/Game/Juli_WB/Blueprints/BP_Leiche.CanBeChopped?` _asbp_leiche)
                    (if (or _returnvalue_3 _returnvalue_4 _returnvalue_5 _returnvalue_6 _returnvalue_2)
                      (`/Game/Juli_WB/Blueprints/BP_Leiche.Chop` _asbp_leiche DeltaSeconds _returnvalue_3 _returnvalue_4 _returnvalue_5 _returnvalue_6 _returnvalue_2)
                      (set `self.isChopping` true)
                      (else
                        (set `self.isChopping` false :!label _label_2)
                        (goto _label :!via `Close`)))
                    (else
                      (goto _label_2))))
                (:`CastFailed`
                  (goto _label_2))))
            (:`CastFailed`
              (goto _label_2))))))))

(fn `DeskFunctions`
  (params (HitActor :type "Actor Object Reference"))
  (bind _holdinglocation (`self.HoldingLocation`))
  (bind _holdingitem (`self.HoldingItem`))
  (bind _holdingitem_2 (`self.HoldingItem`))
  (`|ExecutionSequence`
    (:`then_0`
      (bind _asbp_desk (cast `/Game/Juli_WB/Blueprints/BP_Desk` HitActor))
      (bind _item (`/Game/Juli_WB/Blueprints/BP_Desk.Item` _asbp_desk))
      (`/Engine/EditorBlueprintResources/StandardMacros.IsValid` _item
        (:`Is Valid`
          (`/Engine/EditorBlueprintResources/StandardMacros.IsValid` _holdingitem
            (:`Is Not Valid`
              (`self.K2_DetachFromActor` _item "KeepWorld" "KeepWorld" "KeepWorld")
              (bind _output_get (set `self.HoldingItem` _item))
              (`self.K2_AttachToComponent` _output_get (`self.HoldingLocation`) "None" "SnapToTarget" "SnapToTarget" "KeepWorld" true)
              (set `/Game/Juli_WB/Blueprints/BP_Desk.Item` null _asbp_desk)
              (if (== (`self.HoldingItem`) (`self.Machete`))
                (`SceneComponent.K2_SetWorldRotation` _holdinglocation (struct :`Pitch` 270.0 :`Yaw` 270.0) false false)
                (elif (== (`self.HoldingItem`) (`self.Hammer`))
                  (`SceneComponent.K2_SetWorldRotation` _holdinglocation (struct :`Yaw` 70.0) false false)
                  (elif (== (`self.HoldingItem`) (`self.Saege`))
                    (`SceneComponent.K2_SetWorldRotation` :`self` _holdinglocation)
                    (elif (== (`self.HoldingItem`) (`self.Schere`))
                      (`SceneComponent.K2_SetWorldRotation` :`self` _holdinglocation)
                      (elif (== (`self.HoldingItem`) (`self.Spoon`))
                        (`SceneComponent.K2_SetWorldRotation` :`self` _holdinglocation)))))))))
        (:`Is Not Valid`
          (`/Engine/EditorBlueprintResources/StandardMacros.IsValid` _holdingitem
            (:`Is Valid`
              (`self.K2_DetachFromActor` _holdingitem_2 "KeepWorld" "KeepWorld" "KeepWorld")
              (`self.K2_AttachToComponent` _holdingitem_2 (`/Game/Juli_WB/Blueprints/BP_Desk.ItemLocation` _asbp_desk) "None" "SnapToTarget" "SnapToTarget" "KeepWorld" true)
              (if (== (`self.HoldingItem`) (`self.Machete`))
                (bind _itemlocation (`/Game/Juli_WB/Blueprints/BP_Desk.ItemLocation` _asbp_desk))
                (`SceneComponent.K2_SetWorldRotation` _itemlocation (struct :`Yaw` 30.0 :`Roll` 90.0) false false)
                (elif (== (`self.HoldingItem`) (`self.Hammer`))
                  (`SceneComponent.K2_SetWorldRotation` _itemlocation (struct :`Yaw` 280.0 :`Roll` 90.0) false false)
                  (elif (== (`self.HoldingItem`) (`self.Saege`))
                    (`SceneComponent.K2_SetWorldRotation` :`self` _itemlocation)
                    (elif (== (`self.HoldingItem`) (`self.Schere`))
                      (`SceneComponent.K2_SetWorldRotation` _itemlocation (struct :`Pitch` 90.0 :`Yaw` 90.0 :`Roll` 90.0) false false)
                      (elif (== (`self.HoldingItem`) (`self.Spoon`))
                        (`SceneComponent.K2_SetWorldRotation` :`self` _itemlocation))))))
              (set `/Game/Juli_WB/Blueprints/BP_Desk.Item` _holdingitem_2 _asbp_desk)
              (set `self.HoldingItem` null)
              (`PrimitiveComponent.SetMaterial` (`/Game/Juli_WB/Blueprints/BP_Desk.Cube` _asbp_desk) 0 "/Game/Juli_WB/Assets/Materials/Ablage_7_Blut_3_Mat.Ablage_7_Blut_3_Mat"))))))
    (:`then_1`
      (bind _asbp_item (cast `/Game/Juli_WB/Blueprints/BP_Item` HitActor))
      (`/Engine/EditorBlueprintResources/StandardMacros.IsValid` (`self.HoldingItem`)
        (:`Is Not Valid`
          (bind _sphere (`/Game/Juli_WB/Blueprints/BP_Item.Sphere` _asbp_item))
          (`PrimitiveComponent.SetSimulatePhysics` _sphere false)
          (`PrimitiveComponent.SetCollisionEnabled` _sphere "NoCollision")
          (bind _output_get_2 (set `self.HoldingItem` _asbp_item))
          (`self.K2_AttachToComponent` _output_get_2 (`self.HoldingLocation`) "None" "SnapToTarget" "KeepWorld" "KeepWorld" true))))))

(fn `UserConstructionScript`)